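; GameVariableStorage holds per-player scores and the local player list for a game of up to four players.
; AddScore passes a player index to HandleScore, which adds 10 points and refreshes the CrosshairWidget; index 2 credits Player2Score, leaving Player3Score unincremented.
; ResetScore zeroes all scores.
; EndPlay calls ResetPlayers, which removes local players and their pawns, then opens the results screen level.
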(event `End Play`
  (`self.Reset Players`)
  (`GameplayStatics.OpenLevelBySoftObjectPtr` "/Game/Levels/ResultsScreen.ResultsScreen"))

(event `AddScore`
  (params (ScoringPlayer :type Integer))
  (bind _output_get (set `self.Scoring Player` ScoringPlayer))
  (`self.HandleScore` _output_get))

(event `ResetScore`
  (set `self.Player 1 Score` 0)
  (set `self.Player 2 Score` 0)
  (set `self.Player 3 Score` 0)
  (set `self.Player 4 Score` 0))

(event `Reset Players`
  (bind _localplay (`self.LocalPlay`))
  (for _index (range (+ (+ (`self.NumberOfPlayers`) 1) 1))
    (bind _output (`|GetArrayItem` _localplay _index))
    (bind _playerindex (`TurnBasedBlueprintLibrary.GetMyPlayerIndex` _output))
    (`KismetSystemLibrary.PrintString` (`KismetStringLibrary.BuildString_Int` "" "Player: " _playerindex " Removed"))
    (`GameplayStatics.RemovePlayer` _output true)
    (`KismetArrayLibrary.Array_Remove` _localplay _index)))

(fn `HandleScore`
  (params (`Player Number` :type Integer))
  (if (== `Player Number` 0)
    (set `self.Player 1 Score` (+ (`self.Player 1 Score`) 10))
    (bind _ascrosshair_widget (cast `/Game/Blueprints/UI/CrosshairWidget` (`self.UI`) :!label _label))
    (`/Game/Blueprints/UI/CrosshairWidget.UpdateScore` _ascrosshair_widget)
    (elif (== `Player Number` 1)
      (set `self.Player 2 Score` (+ (`self.Player 2 Score`) 10))
      (goto _label)
      (elif (== `Player Number` 2)
        (set `self.Player 2 Score` (+ (`self.Player 2 Score`) 10))
        (goto _label)
        (elif (== `Player Number` 3)
          (set `self.Player 4 Score` (+ (`self.Player 4 Score`) 10))
          (goto _label))))))