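; Health pickup that restores health to the first-person character when it overlaps the interaction area while active.
; Heal adds the heal value, clamped to the character's Health as maximum, then hides the pickup and deactivates it.
; A Cooldown event re-enables and shows the pickup after a respawn delay.
; Tick spins the pickup visuals around yaw by a fixed step per frame, independent of delta time.
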(event `self.InteractionArea.OnComponentBeginOverlap`
  (params (OverlappedComponent :type "PrimitiveComponent Object Reference") (OtherActor :type "Actor Object Reference") (OtherComp :type "PrimitiveComponent Object Reference") (OtherBodyIndex :type Integer) (bFromSweep :type Boolean) (SweepResult :type "HitResult Structure (by ref)"))
  (if (`self.Active`)
    (`self.Heal` OtherActor)))

(event `Cooldown`
  (`KismetSystemLibrary.Delay` (`self.RespawnTimer`))
  (bind _output_get (set `self.Active` true))
  (`SceneComponent.SetVisibility` (`self.PickupDetails`) _output_get true))

(event `self.ReceiveTick`
  (params (DeltaSeconds :type "Float (single-precision)"))
  (bind _pickupdetails (`self.PickupDetails`))
  (bind (_returnvalue_roll _returnvalue_pitch _returnvalue_yaw) (`KismetMathLibrary.BreakRotator` (`SceneComponent.K2_GetComponentRotation` _pickupdetails)))
  (`SceneComponent.K2_SetWorldRotation` _pickupdetails (`KismetMathLibrary.MakeRotator` 0.0 0.0 (+ _returnvalue_yaw 1.0)) false false))

(fn `Heal`
  (params (PlayerToHeal :type "Actor Object Reference"))
  (bind _asbp_first_person_character (cast `/Game/FPSStarterContent/FirstPerson/Blueprints/BP_FirstPersonCharacter` PlayerToHeal))
  (set `/Game/FPSStarterContent/FirstPerson/Blueprints/BP_FirstPersonCharacter.CurrentHealth` (`KismetMathLibrary.Clamp` (+ (`self.HealValue`) (`/Game/FPSStarterContent/FirstPerson/Blueprints/BP_FirstPersonCharacter.CurrentHealth` _asbp_first_person_character)) 1 (`/Game/FPSStarterContent/FirstPerson/Blueprints/BP_FirstPersonCharacter.Health` _asbp_first_person_character)) _asbp_first_person_character)
  (bind _output_get (set `self.Active` false))
  (`SceneComponent.SetVisibility` (`self.PickupDetails`) _output_get true)
  (`self.Cooldown`))

(fn `UserConstructionScript`)